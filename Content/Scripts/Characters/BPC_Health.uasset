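; Health component for characters that tracks current health and whether the owner is defeated.
; Current health is set to the maximum on BeginPlay.
; DecreaseHealth subtracts incoming damage, clamps health at zero, updates the defeated flag and prints a debug message on each call.
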(event `self.ReceiveBeginPlay`
  (set `self.CurrentHealth` (`self.MaxHealth`)))

(fn `DecreaseHealth`
  (params (IncomingDamage :type "Float (double-precision)"))
  (`KismetSystemLibrary.PrintString` "DO DAMAGE" true true (struct :`R` 1.0 :`G` 0.157344 :`B` 0.277152 :`A` 1.0) 2.0 "DamageNone")
  (set `self.CurrentHealth` (`KismetMathLibrary.FMax` (- (`self.CurrentHealth`) IncomingDamage)))
  (set `self.IsDefeated` (<= (`self.CurrentHealth`) 0.0)))