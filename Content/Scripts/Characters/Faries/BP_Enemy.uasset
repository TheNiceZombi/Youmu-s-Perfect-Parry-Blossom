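; BP_Enemy is an enemy actor that repeatedly fires at the player.
; On BeginPlay it stores BP_Player as its target, waits briefly, then starts AttackPlayer, a delayed self-calling loop.
; Each shot comes from ACObjectPool at the enemy's location, rotated toward the target's current position.
; MoveEnemy and DeactivateEnemy are empty stubs, and an older direct projectile spawn path is left disconnected.
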(event `self.ReceiveBeginPlay`
  (bind _returnvalue (`GameplayStatics.GetActorOfClass` "/Game/Scripts/Characters/Youmu/BP_Player.BP_Player_C"))
  (set `self.My Target` _returnvalue)
  (`KismetSystemLibrary.Delay` 1.0)
  (`self.AttackPlayer`))

(event `Move Enemy`)

(event `AttackPlayer`
  (`/Game/Scripts/Characters/Projectiles/AC_ObjectPool.SpawnFromPool` (`self.AC_ObjectPool`) (`KismetMathLibrary.MakeTransform` (`self.K2_GetActorLocation`) (`KismetMathLibrary.FindLookAtRotation` (`self.K2_GetActorLocation`) (`self.K2_GetActorLocation` (`self.My Target`)))))
  (`KismetSystemLibrary.Delay` 1.0)
  (`self.AttackPlayer`))

(fn `Deactivate_Enemy`)

(fn `UserConstructionScript`)