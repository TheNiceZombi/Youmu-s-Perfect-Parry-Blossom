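; BP_EnemyPath is a spline path actor that moves an array of enemy actors along it in a continuous loop.
; A timeline scaled by TimeLength restarts on finish, driving distance along the spline with a per-index offset that wraps past the end.
; The construction script pre-places the enemies at that spacing.
; Positions use local-space spline locations, tangent-based flipping is unwired, and ActivateRequestedActors is empty.
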(event `self.ReceiveBeginPlay`
  ;[1 1 1] Start Timeline and Set Playrate
  (`TimelineComponent.SetPlayRate` (`self.Timeline`) (/ 1.0 (`self.TimeLength`)))
  (`self.Play_Timeline`))

(event `Play_Timeline`
  (bind _returnvalue (`SplineComponent.GetSplineLength` (`self.Spline`)))
  (bind (_direction _alpha) (`Timeline|Timeline` :!via `PlayFromStart`)
    (:`Update`
      (for (_array_element _array_index) (`self.EnemyType`)
        (bind _output_get (set `self.DistanceAlongSpline` (+ (`KismetMathLibrary.Lerp` 0.0 (`SplineComponent.GetSplineLength` (`self.Spline`)) _alpha) (* (`self.Offset BetweenActors`) _array_index))))
        ;[1 1 1] IF: New offset is Greater than the spline length
        (if (> _output_get _returnvalue)
          (set `self.DistanceAlongSpline` (- (`self.DistanceAlongSpline`) _returnvalue)))
        (`self.K2_SetActorTransform` _array_element (`KismetMathLibrary.MakeTransform` (`SplineComponent.GetLocationAtDistanceAlongSpline` (`self.Spline`) (`self.DistanceAlongSpline`) "Local")) false false)))
    (:`Finished`
      (`self.Play_Timeline`))))

(fn `Activate_RequestedActors`)

(fn `UserConstructionScript`
  (for (_array_element _array_index) (`self.EnemyType`)
    (`self.K2_SetActorTransform` _array_element (`KismetMathLibrary.MakeTransform` (`SplineComponent.GetLocationAtDistanceAlongSpline` (`self.Spline`) (* _array_index (`self.Offset BetweenActors`)) "Local")) false false)))