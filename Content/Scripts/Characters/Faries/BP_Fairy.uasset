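; BP_Fairy is an enemy fairy that repeatedly shoots at the player from BeginPlay onward.
; AttackPlayer fires at once, then plays the FireRate timeline and calls itself when it finishes, using the timeline as the loop delay.
; Fire looks up BP_Player and spawns a short-lived BP_BulletSmall at the fairy's location, rotated toward the player's position at that moment.
; Tick has a StraightSprite branch with no behavior.
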(event `self.ReceiveBeginPlay`
  (`self.AttackPlayer`))

(event `self.ReceiveTick`
  (params (DeltaSeconds :type "Float (single-precision)"))
  (if (`self.StraightSprite`)
    _))

(event `AttackPlayer`
  (`|ExecutionSequence`
    (:`then_0`
      (`self.Fire`))
    (:`then_1`
      (`Timeline|Timeline` :`NewTime` (`self.FireRate`) :!via `PlayFromStart`
        (:`Finished`
          (`self.AttackPlayer`))))))

(fn `Fire`
  (bind _returnvalue (`self.K2_GetActorLocation`))
  (bind _returnvalue_2 (`GameplayStatics.GetActorOfClass` "/Game/Scripts/Characters/Youmu/BP_Player.BP_Player_C"))
  (`|SpawnActorFromClass` "/Game/Scripts/Characters/Projectiles/BP_BulletSmall.BP_BulletSmall_C" (`KismetMathLibrary.MakeTransform` _returnvalue (`KismetMathLibrary.FindLookAtRotation` _returnvalue (`self.K2_GetActorLocation` _returnvalue_2))) "AlwaysSpawn" "MultiplyWithRoot" null 5.0 null))

(fn `UserConstructionScript`)