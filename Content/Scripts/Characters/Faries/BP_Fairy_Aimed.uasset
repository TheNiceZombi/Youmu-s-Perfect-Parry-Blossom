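; BP_Fairy_Aimed is an enemy fairy that repeatedly shoots small bullets aimed at the player's position.
; A self-restarting Timeline, driven by FireRate, calls Fire each cycle while the health component is not defeated, spawning short-lived bullets rotated toward the player.
; On taking damage it reports progress to the player's in-game UI and destroys itself.
; Tick can lock the sprite's world rotation through the StraightSprite flag.
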(event `self.ReceiveBeginPlay`
  (set `/Game/Scripts/Characters/BPC_Health.CurrentHealth` 0.0 (`self.BPC_Health`))
  (`self.AttackPlayer`))

(event `self.ReceiveTick`
  (params (DeltaSeconds :type "Float (single-precision)"))
  (if (`self.StraightSprite`)
    (`SceneComponent.K2_SetWorldRotation` (`self.Sprite`) (struct :`Roll` -90.0) false false)))

(event `AttackPlayer`
  (if (not (`/Game/Scripts/Characters/BPC_Health.IsDefeated` (`self.BPC_Health`)))
    (`Timeline|Timeline` :`NewTime` (`self.FireRate`) :!via `PlayFromStart`
      (:`Finished`
        (`KismetSystemLibrary.PrintString` "Fire")
        (`self.Fire`)
        (`self.AttackPlayer`)))))

(event `self.ReceiveAnyDamage`
  (params (Damage :type "Float (single-precision)") (DamageType :type "DamageType Object Reference") (InstigatedBy :type "Controller Object Reference") (DamageCauser :type "Actor Object Reference"))
  (bind _asbp_player (castclass `/Game/Scripts/Characters/Youmu/BP_Player` "/Game/Scripts/Characters/Youmu/BP_Player.BP_Player_C"))
  (bind _returnvalue (`GameplayStatics.GetActorOfClass` _asbp_player))
  (`KismetSystemLibrary.PrintString` "ADDING PROGRESS")
  (`/Game/Scripts/Characters/Youmu/AC_InGameUI.AddProgress` (`/Game/Scripts/Characters/Youmu/BP_Player.AC_InGameUI` _returnvalue) (> Damage 1.0))
  (`self.K2_DestroyActor`))

(fn `Fire`
  (bind _returnvalue (`self.K2_GetActorLocation`))
  (bind _returnvalue_2 (`GameplayStatics.GetActorOfClass` "/Game/Scripts/Characters/Youmu/BP_Player.BP_Player_C"))
  (`|SpawnActorFromClass` "/Game/Scripts/Characters/Projectiles/BP_BulletSmall.BP_BulletSmall_C" (`KismetMathLibrary.MakeTransform` _returnvalue (`KismetMathLibrary.FindLookAtRotation` _returnvalue (`self.K2_GetActorLocation` _returnvalue_2))) "AlwaysSpawn" "MultiplyWithRoot" null 5.0 null))

(fn `UserConstructionScript`)