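; Actor component that keeps a pool of pre-spawned actors for reuse, filed with the character projectile scripts.
; On BeginPlay it spawns actors of the configured class, passing each a time to live, and marks them not in use.
; SpawnFromPool linearly searches for the first free actor, teleport-free moves it to the requested transform and marks it in use.
; An exhausted pool only prints a failure message rather than growing.
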(event `self.ReceiveBeginPlay`
  (`self.initialize Pool`))

(event `initialize Pool`
  (for _ (range (+ (`self.PoolSize`) 1))
    (bind _returnvalue (`|SpawnActorFromClass` (`self.PooledActorClass`) (`KismetMathLibrary.MakeTransform` (0.0 0.0 0.0)) "AlwaysSpawn" "MultiplyWithRoot" null (`self.Time to Live`) null))
    (`KismetArrayLibrary.Array_AddUnique` (`self.ObjectPool`) _returnvalue)
    (`/Game/Scripts/Characters/Projectiles/BP_PooledActor.SetInUse` _returnvalue false)))

(fn `FindFirstAvailableActor`
  (returns (PooledActor :type "/Game/Scripts/Characters/Projectiles/BP_PooledActor Object Reference"))
  (for _array_element (`self.ObjectPool`)
    (if (not (`/Game/Scripts/Characters/Projectiles/BP_PooledActor.InUse` _array_element))
      (return _array_element))))

(fn `SpawnFromPool`
  (params (SpawnTransform :type "Transform Structure"))
  (returns (PooledActor :type "/Game/Scripts/Characters/Projectiles/BP_PooledActor Object Reference"))
  (bind _pooledactor (`self.FindFirstAvailableActor`))
  (`/Engine/EditorBlueprintResources/StandardMacros.IsValid` _pooledactor
    (:`Is Valid`
      (`Actor.K2_SetActorTransform` _pooledactor SpawnTransform false false)
      (`/Game/Scripts/Characters/Projectiles/BP_PooledActor.SetInUse` _pooledactor true)
      (return _pooledactor))
    (:`Is Not Valid`
      (`KismetSystemLibrary.PrintString` "Failed to Spawn actor from Pool"))))