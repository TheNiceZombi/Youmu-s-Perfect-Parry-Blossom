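; BP_BulletSmall is a small projectile that damages the player on contact.
; On BeginPlay it sets its ProjectileMovement velocity along the actor's forward vector, scaled by Speed.
; When its Sphere overlaps a component tagged PlayerHitBox, it applies a small fixed damage to that component's actor and destroys itself, ignoring other overlaps.
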(event `self.ReceiveBeginPlay`
  (set `MovementComponent.Velocity` (* (`self.GetActorForwardVector`) (`self.speed`)) (`self.ProjectileMovement`)))

(event `self.Sphere.OnComponentBeginOverlap`
  (params (OverlappedComponent :type "PrimitiveComponent Object Reference") (OtherActor :type "Actor Object Reference") (OtherComp :type "PrimitiveComponent Object Reference") (OtherBodyIndex :type Integer) (bFromSweep :type Boolean) (SweepResult :type "HitResult Structure (by ref)"))
  (if (`ActorComponent.ComponentHasTag` OtherComp "PlayerHitBox")
    (`GameplayStatics.ApplyDamage` OtherActor 0.5)
    (`self.K2_DestroyActor`)))

(fn `UserConstructionScript`)