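; BP_ParryBullet is a pooled-style projectile that homes in on an enemy, apparently as a parry counter.
; When set in use, it scans all BP_Enemy actors, intending the nearest, though its comparison favors farther ones, and starts a timeline.
; Tick lerps its location toward that target by the timeline alpha, sweeping and facing it.
; Overlapping an Enemy-tagged actor deals damage and destroys the bullet rather than releasing it.
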(event `self.SetInUse`
  (params (InUse :type Boolean))
  (`parent.SetInUse` InUse)
  (if InUse
    (`|ExecutionSequence`
      (:`then_0`
        ;[1 1 1] GET Nearest Enemy
        (bind _outactors (`GameplayStatics.GetAllActorsOfClass` "/Game/Scripts/Characters/Faries/BP_Enemy.BP_Enemy_C"))
        (for _array_element _outactors
          (bind _returnvalue (`KismetMathLibrary.Vector_Distance` (`self.K2_GetActorLocation`) (`self.K2_GetActorLocation` _array_element)))
          (if (< (`self.Nearest Distance`) (`KismetMathLibrary.Abs` _returnvalue))
            (set `self.Nearest Distance` _returnvalue)
            (set `self.ParryTarget` _array_element))))
      (:`then_1`
        ;[1 1 1] Start Transformation Lerp
        (bind (_direction _travel_lerp) (`Timeline|Timeline` :!via `PlayFromStart`)
          (:`Update`
            (bind _output_get (set `self.Travel Lerp` _travel_lerp))))))))

(event `self.ReceiveBeginPlay`)

(event `self.ReceiveTick`
  (params (DeltaSeconds :type "Float (single-precision)"))
  (bind _returnvalue (`self.K2_GetActorLocation`))
  (bind _returnvalue_2 (`self.K2_GetActorLocation` (`self.ParryTarget`)))
  ;[1 1 1] Move Towards Target
  (`self.K2_SetActorLocation` (`KismetMathLibrary.VLerp` _returnvalue _returnvalue_2 (`self.Travel Lerp`)) true)
  (`self.K2_SetActorRotation` (`KismetMathLibrary.FindLookAtRotation` _returnvalue _returnvalue_2)))

(event `self.ReceiveActorBeginOverlap`
  (params (OtherActor :type "Actor Object Reference"))
  ;[1 1 1] Collision With Enemy
  (if (`self.ActorHasTag` OtherActor "Enemy")
    (`GameplayStatics.ApplyDamage` OtherActor 1.0)
    (`self.K2_DestroyActor`)))

(fn `UserConstructionScript`)