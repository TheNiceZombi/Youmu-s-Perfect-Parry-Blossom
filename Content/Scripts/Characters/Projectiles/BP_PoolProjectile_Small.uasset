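; BP_PoolProjectile_Small is a small pooled projectile that is toggled in and out of use rather than spawned and destroyed.
; SetInUse calls the parent, then either launches it along its forward vector at Speed with particles active, or zeroes velocity and deactivates particles.
; Overlaps check the sphere event's other component for the PlayerHitBox tag and release the projectile on a match; the ApplyDamage node is disconnected, so no damage is dealt here.
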(event `self.SetInUse`
  (params (InUse :type Boolean))
  (`parent.SetInUse` InUse)
  (if InUse
    (set `MovementComponent.Velocity` (* (`self.GetActorForwardVector`) (`self.Speed`)) (`self.ProjectileMovement`))
    (`ActorComponent.Activate` (`self.Particles`) false)
    (else
      (set `MovementComponent.Velocity` (0.0 0.0 0.0) (`self.ProjectileMovement`))
      (`ActorComponent.Deactivate` (`self.Particles`)))))

(event `self.Sphere.OnComponentBeginOverlap`
  (params (OverlappedComponent :type "PrimitiveComponent Object Reference") (OtherActor :type "Actor Object Reference") (OtherComp :type "PrimitiveComponent Object Reference") (OtherBodyIndex :type Integer) (bFromSweep :type Boolean) (SweepResult :type "HitResult Structure (by ref)"))
  (if (`ActorComponent.ComponentHasTag` OtherComp "PlayerHitBox") :!label _label
    (`self.SetInUse` false)))

(event `self.ReceiveActorBeginOverlap`
  (params (OtherActor :type "Actor Object Reference"))
  (goto _label))

(fn `UserConstructionScript`)