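; Parent projectile Blueprint whose bullets the player can parry.
; On BeginPlay it binds to BP_Player's ParryBullets dispatcher; when that fires while the projectile overlaps the player, it calls SpawnParryBullet and marks itself not in use.
; SpawnParryBullet spawns a short-lived BP_ParryBullet at the projectile's location, targeting its stored owner.
; Range and cursor-direction dot-product checks are disconnected or uncalled, so overlap alone decides a parry.
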(event `self.ReceiveBeginPlay`
  (bind _returnvalue (`GameplayStatics.GetActorOfClass` "/Game/Scripts/Characters/Youmu/BP_Player.BP_Player_C"))
  (add `/Game/Scripts/Characters/Youmu/BP_Player.ParryBullets` _returnvalue (delegate `ParryBullets_Event`)))

(event `ParryBullets_Event`
  (params (ParryRange :type "Float (double-precision)") (PerfectParryRadius :type "Float (double-precision)") (AttackWidth :type "Float (double-precision)") (ParryCooldown :type "Float (double-precision)") (Player :type "Actor Object Reference") (Cursor :type "ActorComponent Object Reference"))
  (if (> (`KismetArrayLibrary.Array_Length` (`self.GetOverlappingActors` "/Game/Scripts/Characters/Youmu/BP_Player.BP_Player_C")) 0)
    (`KismetSystemLibrary.PrintString` "Spawn Parry")
    (`self.SpawnParryBullet`)
    (`self.SetInUse` false)))

(fn `Compare Range and Distance`
  (params (B :type "Float (double-precision)") (B2 :type "Float (double-precision)") (B3 :type "Float (double-precision)") (Player :type "Actor Object Reference") (Cursor :type "Actor Object Reference") (A :type "Vector Structure"))
  (returns (ReturnValue :type Boolean) (ReturnValue2 :type Boolean))
  (bind _returnvalue (`self.K2_GetActorLocation` Player))
  (return (> (`KismetMathLibrary.Dot_VectorVector` (`KismetMathLibrary.Normal` _returnvalue) (`KismetMathLibrary.Normal` A)) B3) (< (`KismetMathLibrary.Vector_Distance` _returnvalue (`self.K2_GetActorLocation`)) B)))

(fn `SpawnParryBullet`
  (bind _returnvalue (`|SpawnActorFromClass` "/Game/Scripts/Characters/Projectiles/BP_ParryBullet.BP_ParryBullet_C" (`KismetMathLibrary.MakeTransform` (`self.K2_GetActorLocation`)) "Undefined" "MultiplyWithRoot" null 2.0 null))
  (set `/Game/Scripts/Characters/Projectiles/BP_ParryBullet.ParryTarget` (`self.MyOwner_0`) _returnvalue))

(fn `UserConstructionScript`)