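; AC_InGameUI is a component in the Youmu character folder that manages the main in-game HUD.
; It creates WBP_MainHUD at zero opacity and exposes a fade function.
; AddProgress advances the spring bar, adding a second step on a perfect parry, whose result can fire CollectedAllSpring.
; It also toggles a camera blocker actor's collision, visibility and tick; StartNewEncounter is an empty stub.
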(fn `AddProgress`
  (params (PerfectParry :type Boolean))
  (bind _wbp_springbar (`/Game/UI/Ingame_HUD/WBP_MainHUD.WBP_SpringBar` (`self.Main HUD`)))
  (`/Game/UI/Ingame_HUD/WBP_SpringBar.AddProgress` _wbp_springbar)
  (if PerfectParry
    (bind _completed (`/Game/UI/Ingame_HUD/WBP_SpringBar.AddProgress` _wbp_springbar))
    (if _completed
      (`self.CollectedAllSpring`))))

(fn `CameraObject_Toggle`
  (params (`On/OFF` :type Boolean))
  (bind _camerablockactor (`self.CameraBlockActor`))
  (bind _setcamerablocker (`self.SetCameraBlocker`))
  (`Actor.SetActorEnableCollision` _camerablockactor _setcamerablocker)
  (`Actor.SetActorHiddenInGame` _camerablockactor (not _setcamerablocker))
  (`Actor.SetActorTickEnabled` _camerablockactor _setcamerablocker))

(fn `Fade_UI`
  (params (Alpha :type "Float (double-precision)"))
  (`Widget.SetRenderOpacity` (`self.Main HUD`) Alpha))

(fn `Initialize_UI`
  (bind _returnvalue (`|GenericCreateObject` "/Game/UI/Ingame_HUD/WBP_MainHUD.WBP_MainHUD_C"))
  (bind _output_get (set `self.Main HUD` _returnvalue))
  (`UserWidget.AddToViewport` _output_get 0)
  (`Widget.SetRenderOpacity` _output_get 0.0))

(fn `Start_NewEncounter`
  (params (NewParam :type Boolean)))