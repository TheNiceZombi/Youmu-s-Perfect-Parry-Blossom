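; BP_CameraBlocks is a level-planning actor with four cubes forming an adjustable boundary, presumably for the camera, going by its name.
; The Construction Script offsets the cubes outward in opposing pairs along X and Y by Ratio, so the layout previews in the editor.
; BeginPlay hides the cubes and applies the same relative offsets again, adding to any offset from construction.
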(event `self.ReceiveBeginPlay`
  (bind (_ratio_x _ratio_y) (`KismetMathLibrary.BreakVector4` (`self.Ratio`)))
  (`SceneComponent.SetVisibility` (`self.Cube`) false false)
  (`SceneComponent.SetVisibility` (`self.Cube1`) false false)
  (`SceneComponent.SetVisibility` (`self.Cube2`) false false)
  (`SceneComponent.SetVisibility` (`self.Cube3`) false false)
  (`SceneComponent.K2_AddLocalOffset` (`self.Cube3`) (`KismetMathLibrary.MakeVector` (* _ratio_x -1.0)) false false)
  (`SceneComponent.K2_AddLocalOffset` (`self.Cube1`) (`KismetMathLibrary.MakeVector` _ratio_x) false false)
  (`SceneComponent.K2_AddLocalOffset` (`self.Cube`) (`KismetMathLibrary.MakeVector` 0.0 _ratio_y) false false)
  (`SceneComponent.K2_AddLocalOffset` (`self.Cube2`) (`KismetMathLibrary.MakeVector` 0.0 (* _ratio_y -1.0)) false false))

(fn `UserConstructionScript`
  (bind (_ratio_x _ratio_y) (`KismetMathLibrary.BreakVector4` (`self.Ratio`)))
  (`SceneComponent.K2_AddLocalOffset` (`self.Cube3`) (`KismetMathLibrary.MakeVector` (* _ratio_x -1.0)) false false)
  (`SceneComponent.K2_AddLocalOffset` (`self.Cube1`) (`KismetMathLibrary.MakeVector` _ratio_x) false false)
  (`SceneComponent.K2_AddLocalOffset` (`self.Cube`) (`KismetMathLibrary.MakeVector` 0.0 _ratio_y) false false)
  (`SceneComponent.K2_AddLocalOffset` (`self.Cube2`) (`KismetMathLibrary.MakeVector` 0.0 (* _ratio_y -1.0)) false false))