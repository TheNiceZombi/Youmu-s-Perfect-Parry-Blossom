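; BP_Encounter is a trigger-box level encounter that starts timed enemy waves when the player's hitbox enters it.
; On overlap it broadcasts the defeat quota and camera position (its own location if unset), spawns camera blocks and disables retriggering.
; A Timeline serves as the clock, broadcasting each wave index as playback passes its WaveTiming entry.
; After the Timeline and a delay, it destroys the blocks and signals completion.
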(event `self.ReceiveBeginPlay`
  ;[1 1 1] Set Encounter Time Length
  (`TimelineComponent.SetTimelineLength` (`self.Timeline`) (`self.EncounterTimeLength`)))

(event `self.Box.OnComponentBeginOverlap`
  (params (OverlappedComponent :type "PrimitiveComponent Object Reference") (OtherActor :type "Actor Object Reference") (OtherComp :type "PrimitiveComponent Object Reference") (OtherBodyIndex :type Integer) (bFromSweep :type Boolean) (SweepResult :type "HitResult Structure (by ref)"))
  (bind _returnvalue (`self.K2_GetActorLocation`))
  (bind _defeat_qouta (`self.Defeat Qouta`))
  (bind _camera_position (`self.Camera Position`))
  ;[1 1 1] IF Player Walks into encounter, Start encounter
  (if (`ActorComponent.ComponentHasTag` OtherComp "PlayerHitBox")
    (if (== _camera_position (0.0 0.0 0.0) :`ErrorTolerance` 10.0)
      (`self.StartNewEncounter` _defeat_qouta _returnvalue)
      (bind _returnvalue_2 (`|SpawnActorFromClass` "/Game/Scripts/LevelPlanner/BP_CameraBlocks.BP_CameraBlocks_C" (`KismetMathLibrary.MakeTransform` _returnvalue) "AlwaysSpawn" "MultiplyWithRoot" null null))
      (`KismetSystemLibrary.PrintString` (`KismetStringLibrary.Concat_StrStr` "Spawned: " (`KismetSystemLibrary.GetDisplayName` _returnvalue_2)) true true (struct :`G` 0.66 :`B` 1.0 :`A` 1.0) 10.0)
      (set `self.PlayerBlocks` _returnvalue_2)
      (else
        (`self.StartNewEncounter` _defeat_qouta _camera_position)
        (bind _returnvalue_3 (`|SpawnActorFromClass` "/Game/Scripts/LevelPlanner/BP_CameraBlocks.BP_CameraBlocks_C" (`KismetMathLibrary.MakeTransform` _camera_position) "AlwaysSpawn" "MultiplyWithRoot" null null))
        (`KismetSystemLibrary.PrintString` (`KismetStringLibrary.Concat_StrStr` "Spawned: " (`KismetSystemLibrary.GetDisplayName` _returnvalue_3)) true true (struct :`G` 0.66 :`B` 1.0 :`A` 1.0) 20.0)
        (set `self.PlayerBlocks` _returnvalue_3)))
    (`self.StartEncounter`)))

(event `StartEncounter`
  (bind _returnvalue (`TimelineComponent.GetPlaybackPosition` (`self.Timeline`)))
  ;[1 1 1] START: Playback
  (set `PrimitiveComponent.bGenerateOverlapEvents` false (`self.Box`))
  (`Timeline|Timeline`
    (:`Update`
      (`KismetSystemLibrary.PrintString` (`KismetStringLibrary.Concat_StrStr` "Level_Timer: " (`KismetStringLibrary.Conv_DoubleToString` _returnvalue)) true true (struct :`R` 0.98284 :`G` 0.156186 :`B` 1.0 :`A` 1.0) 2.0 "SpawnTimer")
      ;[1 1 1] When Playback reacher a number in the Wave Array: SPAWN Wave of enemies
      (`self.SpawnWave` _returnvalue))
    (:`Finished`
      ;[1 1 1] END Encounter Event
      (`KismetSystemLibrary.K2_SetTimerDelegate` (delegate `EncounterFinished`) (`self.FinishDelay`)))))

(event `EncounterFinished`
  ;[1 1 1] END Encounter Event
  (set `self.Completed` true)
  (`self.K2_DestroyActor` (`self.PlayerBlocks`))
  (`self.EncounterFinish`))

(fn `SpawnWave`
  (params (Time :type "Float (double-precision)"))
  (returns (NewParam :type Name))
  (bind _returnvalue (`KismetStringLibrary.Conv_IntToString` (`self.CurrentWave`)))
  (bind _returnvalue_2 (`KismetSystemLibrary.MakeLiteralName` (`KismetStringLibrary.Conv_StringToName` _returnvalue)))
  ;[1 1 1] IF: Timing matches the next wave timing
  (if (> Time (`|GetArrayItem` (`self.WaveTiming`) (`self.CurrentWave`)))
    ;[1 1 1] IF: Current Wave is less than Array Length
    (if (< (`self.CurrentWave`) (`KismetArrayLibrary.Array_Length` (`self.WaveTiming`)))
      ;[1 1 1] Call Event to everyone with Tag Wave_x
      (`self.StartWave` _returnvalue_2)
      (`KismetSystemLibrary.PrintString` (`KismetStringLibrary.Concat_StrStr` "Spawning: " (`KismetStringLibrary.Concat_StrStr` "Wave_" _returnvalue)) true true (struct :`R` 1.0 :`B` 0.802272 :`A` 1.0) 2.0 "SpawnWave")
      ;[1 1 1] Increment to Next Wave
      (`/Engine/EditorBlueprintResources/StandardMacros.IncrementInt` (`self.CurrentWave`)
        (:`  `
          (return _returnvalue_2))))))

(fn `UserConstructionScript`)