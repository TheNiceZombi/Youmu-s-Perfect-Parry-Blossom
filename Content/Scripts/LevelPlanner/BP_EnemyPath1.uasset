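; Enemy path actor that spawns a wave of enemies and moves them along its spline.
; On EncounterControl's StartWave call with a matching WaveTag, it spawns every class in EnemyArray and plays a timeline scaled to TimeLength.
; Each update maps SpeedCurve to spline distance, staggering enemies by index times TimeBetweenActors, and writes truncated FireCurve values to each BP_EnemyParent's FireRate.
; Surviving enemies are destroyed when the timeline finishes.
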(event `self.ReceiveBeginPlay`
  (set `self.Tags` (`self.WaveTag`))
  ;[1 1 1] LISTEN FOR CALL: Start Wave
  (add `/Game/Scripts/LevelPlanner/BP_Encounter.StartWave` (`self.EncounterControl`) (delegate `StartWave_Event`)))

(event `StartWave_Event`
  (params (NewParam :type Name))
  ;[1 1 1] LISTEN FOR CALL: Start Wave
  (if (> (`KismetArrayLibrary.Array_Find` (`self.WaveTag`) NewParam) -1)
    (`|ExecutionSequence`
      (:`then_0`
        ;[1 1 1] Spawn all Actors
        (for _array_element (`self.EnemyArray`)
          (bind _returnvalue (`|SpawnActorFromClass` _array_element (`KismetMathLibrary.MakeTransform` (0.0 0.0 0.0)) "AlwaysSpawn" "MultiplyWithRoot" null null))
          (`KismetSystemLibrary.PrintString` (`KismetStringLibrary.Concat_StrStr` "Spawning: " (`KismetSystemLibrary.GetDisplayName` _returnvalue)))
          (`KismetArrayLibrary.Array_AddUnique` (`self.ActorArray`) _returnvalue))
        ;[1 1 1] Start Timeline and Set Playrate
        (`TimelineComponent.SetPlayRate` (`self.Timeline`) (/ 1.0 (`self.TimeLength`)))
        (`self.Play_Timeline`)))))

(event `Play_Timeline`
  (bind (_direction _alpha) (`Timeline|Timeline` :!via `PlayFromStart`)
    (:`Update`
      (set `self.FireRate` (`KismetMathLibrary.GetRuntimeFloatCurveValue` (`self.FireCurve`) _alpha))
      (for (_array_element _array_index) (`self.ActorArray`)
        (set `self.DistanceAlongSpline` (`KismetMathLibrary.Lerp` 0.0 (`SplineComponent.GetSplineLength` (`self.Spline`)) (`KismetMathLibrary.FMax` (- (`KismetMathLibrary.GetRuntimeFloatCurveValue` (`self.SpeedCurve`) _alpha) (* _array_index (`self.TimeBetweenActors`))))))
        (`/Engine/EditorBlueprintResources/StandardMacros.IsValid` _array_element
          (:`Is Valid`
            (`self.K2_SetActorTransform` _array_element (`KismetMathLibrary.MakeTransform` (+ (`self.K2_GetActorLocation`) (`SplineComponent.GetLocationAtDistanceAlongSpline` (`self.Spline`) (`self.DistanceAlongSpline`) "Local"))) false false)
            (`/Engine/EditorBlueprintResources/StandardMacros.IsValid` _array_element
              (:`Is Valid`
                (bind _asbp_enemy_parent (cast `/Game/Scripts/Characters/Faries/BP_EnemyParent` _array_element))
                (set `/Game/Scripts/Characters/Faries/BP_EnemyParent.FireRate` (`KismetMathLibrary.Conv_IntToDouble` (`KismetMathLibrary.FTrunc` (`self.FireRate`))) _asbp_enemy_parent)))))))
    (:`Finished`
      ;[1 0.04161 0.05156] WHEN FINISHED: DELETE ALL ENEMIES
      (for _array_element_2 (`self.ActorArray`)
        (`/Engine/EditorBlueprintResources/StandardMacros.IsValid` _array_element_2
          (:`Is Valid`
            (`self.K2_DestroyActor` _array_element_2)))))))

(event `SpawnEnemy`)

(fn `Activate_RequestedActors`)

(fn `UserConstructionScript`)