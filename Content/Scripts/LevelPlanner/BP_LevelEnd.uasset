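; BP_LevelEnd is a level exit trigger that records spring collection per encounter and shows the victory screen.
; On BeginPlay it binds to the player UI's all-springs-collected event and every BP_Encounter's start and finish events.
; Each finished encounter stores the collected flag in completion order, then resets it.
; Box overlap passes that array and the next level name to WBP_Victory, starts a timeline, then switches to UI-only input after a short delay.
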(event `CollectedAllSpring_Event`
  ;[1 1 1] LISTEN FOR: Collected Spring
  (bind _output_get (set `self.SpringCollected` true))
  (`KismetSystemLibrary.PrintString` (`KismetStringLibrary.Concat_StrStr` "CALL: Recieve spring: " (`KismetStringLibrary.Conv_BoolToString` _output_get)) true true (struct :`R` 0.308644 :`G` 1.0 :`B` 0.318043 :`A` 1.0) 10.0))

(event `self.ReceiveBeginPlay`
  (`|ExecutionSequence`
    (:`then_0`
      ;[1 1 1] LISTEN FOR: Collected Spring
      (bind _asac_in_game_ui (castclass `/Game/Scripts/Characters/Youmu/AC_InGameUI` "/Game/Scripts/Characters/Youmu/AC_InGameUI.AC_InGameUI_C"))
      (bind _asbp_player (castclass `/Game/Scripts/Characters/Youmu/BP_Player` "/Game/Scripts/Characters/Youmu/BP_Player.BP_Player_C"))
      (bind _returnvalue (`GameplayStatics.GetActorOfClass` _asbp_player))
      (add `/Game/Scripts/Characters/Youmu/AC_InGameUI.CollectedAllSpring` (`self.GetComponentByClass` _returnvalue _asac_in_game_ui) (delegate `CollectedAllSpring_Event`)))
    (:`then_1`
      ;[1 1 1] LISTEN: For Encounter Event
      (bind _asbp_encounter (castclass `/Game/Scripts/LevelPlanner/BP_Encounter` "/Game/Scripts/LevelPlanner/BP_Encounter.BP_Encounter_C"))
      (bind _outactors (`GameplayStatics.GetAllActorsOfClass` _asbp_encounter))
      (bind _output_get (set `self.NumberOfEncounter` (`KismetArrayLibrary.Array_Length` _outactors)))
      (`KismetArrayLibrary.Array_Resize` (`self.EncounterSpringCollected`) _output_get)
      (for _array_element _outactors
        (add `/Game/Scripts/LevelPlanner/BP_Encounter.StartNewEncounter` _array_element (delegate `StartNewEncounter_Event`))
        (add `/Game/Scripts/LevelPlanner/BP_Encounter.EncounterFinish` _array_element (delegate `EncounterFinish_Event`))))))

(event `StartNewEncounter_Event`
  (params (DefeatQouta :type Integer) (CameraPosition :type "Vector Structure")))

(event `EncounterFinish_Event`
  (`self.Save CollectedSpring`))

(event `ENDLevel`
  (`|ExecutionSequence`
    (:`then_0`
      (bind _returnvalue (`|GenericCreateObject` "/Game/UI/Victory_Menu/WBP_Victory.WBP_Victory_C"))
      (set `/Game/UI/Victory_Menu/WBP_Victory.NextLevelName` (`self.NextLevel`) _returnvalue)
      (set `/Game/UI/Victory_Menu/WBP_Victory.SpringCollection` (`self.EncounterSpringCollected`) _returnvalue)
      (`UserWidget.AddToViewport` _returnvalue 0)
      (`KismetSystemLibrary.Delay` 0.5)
      (`WidgetBlueprintLibrary.SetInputMode_UIOnlyEx` (`GameplayStatics.GetPlayerController` 0) null)
      (set `PrimitiveComponent.bGenerateOverlapEvents` false (`self.Box`)))
    (:`then_1`
      (`Timeline|Timeline` :!via `PlayFromStart`))))

(event `self.Box.OnComponentBeginOverlap`
  (params (OverlappedComponent :type "PrimitiveComponent Object Reference") (OtherActor :type "Actor Object Reference") (OtherComp :type "PrimitiveComponent Object Reference") (OtherBodyIndex :type Integer) (bFromSweep :type Boolean) (SweepResult :type "HitResult Structure (by ref)"))
  (`self.ENDLevel`))

(fn `Save CollectedSpring`
  (bind _encountersfinished (`self.EncountersFinished`))
  (bind _springcollected (`self.SpringCollected`))
  (`KismetSystemLibrary.PrintString` (`KismetStringLibrary.Concat_StrStr` "SpringCollected: " (`KismetStringLibrary.Conv_BoolToString` _springcollected)) true true (struct :`R` 1.0 :`G` 0.826232 :`A` 1.0) 10.0)
  (`KismetArrayLibrary.Array_Set` (`self.EncounterSpringCollected`) _encountersfinished _springcollected true)
  (`/Engine/EditorBlueprintResources/StandardMacros.IncrementInt` _encountersfinished
    (:`  `
      (set `self.SpringCollected` false))))

(fn `UserConstructionScript`)