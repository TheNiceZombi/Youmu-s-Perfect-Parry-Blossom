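; Level planner that triggers numbered waves at set times during a level.
; A Timeline started on BeginPlay acts as the level clock, passing its track value to SpawnWave on every update.
; When that value exceeds the current WaveTiming entry, SpawnWave calls the StartWave dispatcher with a "Wave_N" name and increments CurrentWave.
; Keyed debug prints show the timer and each triggered wave.
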(event `self.ReceiveBeginPlay`
  (bind (_direction _newtrack_0) (`Timeline|Timeline`)
    (:`Update`
      (`KismetSystemLibrary.PrintString` (`KismetStringLibrary.Concat_StrStr` "Level_Timer: " (`KismetStringLibrary.Conv_DoubleToString` _newtrack_0)) true true (struct :`R` 0.98284 :`G` 0.156186 :`B` 1.0 :`A` 1.0) 2.0 "SpawnTimer")
      (`self.SpawnWave` _newtrack_0))))

(fn `SpawnWave`
  (params (Time :type "Float (double-precision)"))
  (returns (NewParam :type Name))
  (bind _returnvalue (`KismetStringLibrary.Concat_StrStr` "Wave_" (`KismetStringLibrary.Conv_IntToString` (`self.CurrentWave`))))
  (bind _returnvalue_2 (`KismetSystemLibrary.MakeLiteralName` (`KismetStringLibrary.Conv_StringToName` _returnvalue)))
  ;[1 1 1] IF: Timing matches the next wave timing
  (if (> Time (`|GetArrayItem` (`self.WaveTiming`) (`self.CurrentWave`)))
    ;[1 1 1] IF: Current Wave is less than Array Length
    (if (< (`self.CurrentWave`) (`KismetArrayLibrary.Array_Length` (`self.WaveTiming`)))
      ;[1 1 1] Call Event to everyone with Tag Wave_x
      (`self.StartWave` _returnvalue_2)
      (`KismetSystemLibrary.PrintString` (`KismetStringLibrary.Concat_StrStr` "Spawning: " _returnvalue) true true (struct :`R` 1.0 :`B` 0.802272 :`A` 1.0) 2.0 "SpawnWave")
      ;[1 1 1] Increment to Next Wave
      (`/Engine/EditorBlueprintResources/StandardMacros.IncrementInt` (`self.CurrentWave`)
        (:`  `
          (return _returnvalue_2))))))

(fn `UserConstructionScript`)